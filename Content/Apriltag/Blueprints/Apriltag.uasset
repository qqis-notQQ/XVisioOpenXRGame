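; Actor that follows an XVisio AprilTag in an XR scene, matching the tag's pose every frame.
; Tick fixes the scale at 0.16, reads tag 0 from the XVisio stream world subsystem, and applies its position and quaternion-derived rotation.
; Unconnected nodes hold a non-streaming variant using the XR subsystem with explicit tag detection, plus stray SLAM map calls.
; The B-key input event is empty.
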(event Input|EnhancedActionEvents|EnhancedInputActionIA_B_Key
  (params (ActionValue :type Boolean) (ElapsedSeconds :type Float%20%28double-precision%29) (TriggeredSeconds :type Float%20%28double-precision%29) (InputAction :type Input%20Action%20Object%20Reference :default "/Game/input/Actions/IA_B_Key.IA_B_Key")))

(event EventBeginPlay)

(event Collision|EventActorBeginOverlap
  (params (OtherActor :type Actor%20Object%20Reference)))

(event EventTick
  (params (DeltaSeconds :type Float%20%28single-precision%29))
  ;[1 0.2892 0.5653] 串流
  (Utilities|FlowControl|Sequence
    (:then_0
      (Transformation|SetActorScale3D "0.160000,0.160000,0.160000"))
    (:then_1
      (bind (_outtagid _outposition _outorientation _outquaternion) (Class|XVisioStreamWorldSubsystem|GetApriltagData (Subsystems|GetXVisioStreamWorldSubsystem)))
      (Transformation|SetActorLocation _outposition false false)
      (Transformation|SetActorRotation (Class|KismetMathLibrary|QuatRotator _outquaternion)))))

(fn ConstructionScript)